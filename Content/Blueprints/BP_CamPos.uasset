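; BP_CamPos is a one-shot cutscene camera that takes the view from the wind pawn when MoveCamera is called.
; CameraMovement flags the pawn, blends to this actor while blocking input, and optionally eases the camera to the Destination transform.
; The Sequence destroys any assigned DestroyWall once that timed shot starts.
; The view then blends back to the player, the flag clears, the actor destroys itself and input is restored.
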(event Custom|Move%20Camera
  (bind _destroywall (Variables|Default|GetDestroyWall))
  (Utilities|FlowControl|Sequence
    (:then_0)
    (:then_1
      (|CameraMovement))
    (:then_3
      (Utilities|IsValid _destroywall
        (:Is%20Valid
          (Actor|DestroyActor _destroywall))))))

(event EventBeginPlay
  (Variables|Default|SetSecondCameraTranform (Transformation|GetRelativeTransform (Variables|Default|GetDestination)))
  (bind _asbp_pawn_wind (Utilities|Casting|CastToBP_Pawn_Wind (Game|Player|GetPlayerPawn 0)))
  (Variables|Default|SetAsBPPawnWind _asbp_pawn_wind))

(fn ConstructionScript)