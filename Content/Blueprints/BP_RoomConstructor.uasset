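; BP_RoomConstructor records the actors of a level as a room layout and respawns copies at the constructor's transform.
; EnlistActors resets its own transform, gathers every Actor, strips some auto-generated ones and the last array entry, then stores transforms and BP_DummyCube mesh scales.
; SpawnEnlisteds spawns each stored class at a composed transform and reapplies cube scales.
; Separate events delete the copies or refresh their scales.
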(event Custom|EnlistActors
  (Transformation|SetActorTransform (Math|Transform|MakeTransform "0, 0, 0" "0, 0, 0" "1.000000,1.000000,1.000000"))
  (Utilities|Array|Clear (Variables|Default|GetActorsInRoomEnlisted))
  (Utilities|Array|Clear (Variables|Default|GetActorsTransforms))
  (Utilities|Array|Clear (Variables|Default|GetMeshScale))
  (bind _outactors (Actor|GetAllActorsOfClass "/Script/Engine.Actor"))
  (bind _output_get (Variables|Default|SetActorsInRoomEnlisted _outactors))
  (CallFunction|RemoveAutoGenerates _output_get)
  (for _array_element (Variables|Default|GetActorsInRoomEnlisted)
    (Utilities|Array|Add (Variables|Default|GetActorsTransforms) (Transformation|GetActorTransform _array_element))
    (bind _asbp_dummy_cube (Utilities|Casting|CastToBP_DummyCube _array_element)
      (:then
        (Utilities|Array|Add (Variables|Default|GetMeshScale) (Variables|/Game/Blueprints/BP_DummyCube.BP_DummyCube_C|GetMeshScale _asbp_dummy_cube)))
      (:CastFailed
        (Utilities|Array|Add (Variables|Default|GetMeshScale) "1.000000,1.000000,1.000000")))))

(event Custom|SpawnEnlisteds
  (Utilities|Array|Clear (Variables|Default|GetActorsInRoomSpawned))
  (for (_array_element _array_index) (Variables|Default|GetActorsInRoomEnlisted)
    (bind _returnvalue (Game|SpawnActorfromClass (Utilities|GetClass _array_element) (Math|Transform|ComposeTransforms (Utilities|Array|Get(acopy) (Variables|Default|GetActorsTransforms) _array_index) (Transformation|GetActorTransform)) "Undefined" 0 0))
    (Utilities|Array|Add (Variables|Default|GetActorsInRoomSpawned) _returnvalue)
    (for (_array_element_2 _array_index_2) (Variables|Default|GetActorsInRoomSpawned)
      (bind _asbp_dummy_cube (Utilities|Casting|CastToBP_DummyCube _array_element_2))
      (Variables|/Game/Blueprints/BP_DummyCube.BP_DummyCube_C|SetMeshScale _asbp_dummy_cube (Utilities|Array|Get(acopy) (Variables|Default|GetMeshScale) _array_index_2))
      (CallFunction|RefreshSpawnedMeshScale))))

(event Custom|DeleteSpawnedActors
  (for _array_element (Variables|Default|GetActorsInRoomSpawned)
    (Actor|DestroyActor _array_element))
  (Utilities|Array|Clear (Variables|Default|GetActorsInRoomSpawned)))

(event Custom|RefreshSpawnedMeshScale
  (for (_array_element _array_index) (Variables|Default|GetActorsInRoomSpawned)
    (bind _asbp_dummy_cube (Utilities|Casting|CastToBP_DummyCube _array_element))
    (Default|RefreshMeshScale _asbp_dummy_cube (Utilities|Array|Get(acopy) (Variables|Default|GetMeshScale) _array_index))))

(fn ConstructionScript)

(fn RemoveActorfromArraybyClass
  (params (ActorClass :type Actor%20Class%20Reference) (TargetArray :type Array%20of%20Actor%20Object%20References))
  (bind _returnvalue (Actor|GetActorOfClass ActorClass))
  (Utilities|Array|RemoveItem TargetArray _returnvalue))

(fn RemoveAutoGenerates
  (params (InputPin :type Array%20of%20Actor%20Object%20References))
  (CallFunction|RemoveActorfromArraybyClass "BP_RoomConstructor_C" InputPin)
  (CallFunction|RemoveActorfromArraybyClass "/Script/Engine.DirectionalLight" InputPin)
  (CallFunction|RemoveActorfromArraybyClass "/Script/Engine.Brush" InputPin)
  (CallFunction|RemoveActorfromArraybyClass "/Script/Engine.DefaultPhysicsVolume" InputPin)
  (CallFunction|RemoveActorfromArraybyClass "/Script/NavigationSystem.AbstractNavData" InputPin)
  (CallFunction|RemoveActorfromArraybyClass "/Script/Engine.WorldSettings" InputPin)
  (CallFunction|RemoveActorfromArraybyClass "/Script/Engine.SkyLight" InputPin)
  (Utilities|Array|RemoveIndex InputPin (- (Utilities|Array|Length InputPin) 1)))