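; Flower actor that reacts once when the wind pawn passes through it, feeding a per-set flower count.
; On BeginPlay it finds the sound player and flower counter in the level, then registers its FlowerSet tag with the counter unless that tag is "False".
; When BP_Pawn_Wind overlaps its Box, it plays the flower sound, decrements the count for its set and destroys the Box to prevent retriggering.
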(event OnComponentBeginOverlap(Box)
  (params (OverlappedComponent :type Primitive%20Component%20Object%20Reference) (OtherActor :type Actor%20Object%20Reference) (OtherComp :type Primitive%20Component%20Object%20Reference) (OtherBodyIndex :type Integer) (bFromSweep :type Boolean) (SweepResult :type Hit%20Result%20Structure%20%28by%20ref%29))
  (Utilities|Casting|CastToBP_Pawn_Wind OtherActor)
  (Default|PlayFlowerSound (Variables|Default|GetSoundPlayer))
  (Default|FlowerMinusOne (Variables|Default|GetCounter) (GameplayTags|GetTagName (Variables|Default|GetFlowerSet)))
  (Components|DestroyComponent (Variables|Default|GetBox)))

(event EventBeginPlay
  (bind _flowerset (Variables|Default|GetFlowerSet))
  (bind _returnvalue (GameplayTags|GetTagName _flowerset))
  (bind _returnvalue_2 (Actor|GetActorOfClass "/Game/Blueprints/BP_SoundPlayer.BP_SoundPlayer_C"))
  (Variables|Default|SetSoundPlayer _returnvalue_2)
  (bind _returnvalue_3 (Actor|GetActorOfClass "/Game/Blueprints/BP_CountingFlower.BP_CountingFlower_C"))
  (bind _output_get (Variables|Default|SetCounter _returnvalue_3))
  (if (not (== _returnvalue "False"))
    (Default|EnlistFlowerSets _output_get _returnvalue)))

(fn ConstructionScript)