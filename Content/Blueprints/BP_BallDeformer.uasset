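; BP_BallDeformer is a deformer component that supplies a deformation capsule for its owning actor, apparently a ball.
; It overrides the deform-capsule query to sweep one capsule from the owner's current location back to the location cached at the previous query, covering the path moved in between.
; Capsule radius is Radius times ActorScale, and both ends carry the owner's velocity at full strength.
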(event EventBeginPlay
  (|CallParentFunction)
  (Variables|Default|SetPrevLocation (Transformation|GetActorLocation (Components|GetOwner))))

(fn BPGetDeformCapsules
  (bind _returnvalue (Components|GetOwner))
  (bind _returnvalue_2 (Transformation|GetActorLocation _returnvalue))
  (bind _returnvalue_3 (Transformation|GetVelocity _returnvalue))
  (bind _array (Utilities|Array|MakeArray (Math|Vector4|MakeVector4 (.x _returnvalue_3) (.y _returnvalue_3) (.z _returnvalue_3) 1.0)))
  (Variables|Default|SetYeeto (* (Variables|Default|GetActorScale) (Variables|Default|GetRadius)))
  (Variables|Default|SetOutEndLocationAndRadius (Utilities|Array|MakeArray (Math|Vector4|MakeVector4 (.x (Variables|Default|GetPrevLocation)) (.y (Variables|Default|GetPrevLocation)) (.z (Variables|Default|GetPrevLocation)) (Variables|Default|GetYeeto))))
  (Variables|Default|SetPrevLocation (Transformation|GetActorLocation (Components|GetOwner)))
  (return (Utilities|Array|MakeArray (Math|Vector4|MakeVector4 (.x _returnvalue_2) (.y _returnvalue_2) (.z _returnvalue_2) (Variables|Default|GetYeeto))) (Variables|Default|GetOutEndLocationAndRadius) _array _array))