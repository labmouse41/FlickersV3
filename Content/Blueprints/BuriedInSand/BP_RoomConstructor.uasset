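; BP_RoomConstructor is an editor-style room tool that records a level's actors as a room layout and respawns them relative to its own transform.
; EnlistActors resets its transform, gathers all actors minus some auto-generated ones, and saves references, transforms and BP_DummyCube mesh scales to a BP_RoomData save slot.
; SpawnEnlisteds loads that slot, spawns and attaches copies, reapplies cube scales and sets the Box extent from their combined bounds.
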(event Custom|EnlistActors
  (Transformation|SetActorTransform (Math|Transform|MakeTransform "0, 0, 0" "0, 0, 0" "1.000000,1.000000,1.000000"))
  (bind _returnvalue (SaveGame|LoadGamefromSlot (Variables|Default|GetDataStorageSlotName)))
  (bind _asbp_room_data (Utilities|Casting|CastToBP_RoomData _returnvalue)
    (:then
      (Variables|Default|SetDataStorage _asbp_room_data))
    (:CastFailed
      (bind _returnvalue_2 (SaveGame|CreateSaveGameObject "/Game/Blueprints/BuriedInSand/BP_RoomData.BP_RoomData_C"))
      (Variables|Default|SetDataStorage _returnvalue_2)))
  (CallFunction|ClearLists)
  (bind _outactors (Actor|GetAllActorsOfClass "/Script/Engine.Actor"))
  (bind _output_get (Variables|Default|SetActorsInRoomEnlisted _outactors))
  (CallFunction|RemoveAutoGenerates _output_get)
  (Variables|/Game/Blueprints/BuriedInSand/BP_RoomData.BP_RoomData_C|SetActorList (Variables|Default|GetDataStorage) (Variables|Default|GetActorsInRoomEnlisted))
  (for _array_element (Variables|/Game/Blueprints/BuriedInSand/BP_RoomData.BP_RoomData_C|GetActorList (Variables|Default|GetDataStorage))
    (Utilities|Array|Add (Variables|Default|GetActorsTransforms) (Transformation|GetActorTransform _array_element))
    (Utilities|Array|Add (Variables|/Game/Blueprints/BuriedInSand/BP_RoomData.BP_RoomData_C|GetTransformList (Variables|Default|GetDataStorage)) (Transformation|GetActorTransform _array_element))
    (bind _asbp_dummy_cube (Utilities|Casting|CastToBP_DummyCube _array_element)
      (:then
        (Utilities|Array|Add (Variables|Default|GetMeshScale) (Variables|/Game/Blueprints/BuriedInSand/BP_DummyCube.BP_DummyCube_C|GetMeshScale _asbp_dummy_cube))
        (Utilities|Array|Add (Variables|/Game/Blueprints/BuriedInSand/BP_RoomData.BP_RoomData_C|GetMeshScaleList (Variables|Default|GetDataStorage)) (Variables|/Game/Blueprints/BuriedInSand/BP_DummyCube.BP_DummyCube_C|GetMeshScale _asbp_dummy_cube)))
      (:CastFailed
        (Utilities|Array|Add (Variables|Default|GetMeshScale) "1.000000,1.000000,1.000000")
        (Utilities|Array|Add (Variables|/Game/Blueprints/BuriedInSand/BP_RoomData.BP_RoomData_C|GetMeshScaleList (Variables|Default|GetDataStorage)) "1.000000,1.000000,1.000000")))
    (SaveGame|SaveGametoSlot (Variables|Default|GetDataStorage) (Variables|Default|GetDataStorageSlotName))))

(event Custom|SpawnEnlisteds
  (CallFunction|DeleteSpawnedActors)
  (bind _returnvalue (SaveGame|LoadGamefromSlot (Variables|Default|GetDataStorageSlotName)))
  (bind _asbp_room_data (Utilities|Casting|CastToBP_RoomData _returnvalue))
  (Variables|Default|SetDataStorage _asbp_room_data)
  (Utilities|Array|Clear (Variables|Default|GetActorsInRoomSpawned))
  (for (_array_element _array_index) (Variables|/Game/Blueprints/BuriedInSand/BP_RoomData.BP_RoomData_C|GetActorList (Variables|Default|GetDataStorage))
    (bind _returnvalue_2 (Game|SpawnActorfromClass (Utilities|GetClass _array_element) (Math|Transform|ComposeTransforms (Utilities|Array|Get(acopy) (Variables|/Game/Blueprints/BuriedInSand/BP_RoomData.BP_RoomData_C|GetTransformList (Variables|Default|GetDataStorage)) _array_index) (Transformation|GetActorTransform)) "Undefined" "SelectDefaultAtRuntime" 0 0))
    (Utilities|Array|Add (Variables|Default|GetActorsInRoomSpawned) _returnvalue_2))
  (for (_array_element_2 _array_index_2) (Variables|Default|GetActorsInRoomSpawned)
    (Transformation|AttachActorToActor _array_element_2 self "None" "KeepWorld" "KeepWorld" "KeepWorld" false)
    (bind _asbp_dummy_cube (Utilities|Casting|CastToBP_DummyCube _array_element_2))
    (Variables|/Game/Blueprints/BuriedInSand/BP_DummyCube.BP_DummyCube_C|SetMeshScale _asbp_dummy_cube (Utilities|Array|Get(acopy) (Variables|/Game/Blueprints/BuriedInSand/BP_RoomData.BP_RoomData_C|GetMeshScaleList (Variables|Default|GetDataStorage)) _array_index_2))
    (CallFunction|RefreshSpawnedMeshScale))
  (bind _boxextent (Collision|GetActorArrayBounds (Variables|Default|GetActorsInRoomSpawned)))
  (Components|Box|SetBoxExtent (Variables|Default|GetBox) _boxextent true))

(event Custom|DeleteSpawnedActors
  (for _array_element (Variables|Default|GetActorsInRoomSpawned)
    (Actor|DestroyActor _array_element))
  (Utilities|Array|Clear (Variables|Default|GetActorsInRoomSpawned)))

(event Custom|RefreshSpawnedMeshScale
  (for (_array_element _array_index) (Variables|Default|GetActorsInRoomSpawned)
    (bind _asbp_dummy_cube (Utilities|Casting|CastToBP_DummyCube _array_element))
    (Default|RefreshMeshScale _asbp_dummy_cube (Utilities|Array|Get(acopy) (Variables|Default|GetMeshScale) _array_index))
    (Development|PrintString (Utilities|String|ToString(Vector) (Utilities|Array|Get(acopy) (Variables|Default|GetMeshScale) _array_index)) true true "(R=0.000000,G=0.660000,B=1.000000,A=1.000000)" 11.0)))

(event Custom|ClearLists
  (Utilities|Array|Clear (Variables|Default|GetActorsInRoomEnlisted))
  (Utilities|Array|Clear (Variables|Default|GetActorsTransforms))
  (Utilities|Array|Clear (Variables|Default|GetMeshScale))
  (Utilities|Array|Clear (Variables|/Game/Blueprints/BuriedInSand/BP_RoomData.BP_RoomData_C|GetActorList (Variables|Default|GetDataStorage)))
  (Utilities|Array|Clear (Variables|/Game/Blueprints/BuriedInSand/BP_RoomData.BP_RoomData_C|GetTransformList (Variables|Default|GetDataStorage)))
  (Utilities|Array|Clear (Variables|/Game/Blueprints/BuriedInSand/BP_RoomData.BP_RoomData_C|GetMeshScaleList (Variables|Default|GetDataStorage))))

(fn ConstructionScript)

(fn RemoveActorfromArraybyClass
  (params (ActorClass :type Actor%20Class%20Reference) (TargetArray :type Array%20of%20Actor%20Object%20References))
  (bind _returnvalue (Actor|GetActorOfClass ActorClass))
  (Utilities|Array|RemoveItem TargetArray _returnvalue))

(fn RemoveAutoGenerates
  (params (InputPin :type Array%20of%20Actor%20Object%20References))
  (CallFunction|RemoveActorfromArraybyClass "BP_RoomConstructor_C" InputPin)
  (CallFunction|RemoveActorfromArraybyClass "/Script/Engine.DirectionalLight" InputPin)
  (CallFunction|RemoveActorfromArraybyClass "/Script/Engine.Brush" InputPin)
  (CallFunction|RemoveActorfromArraybyClass "/Script/Engine.DefaultPhysicsVolume" InputPin)
  (CallFunction|RemoveActorfromArraybyClass "/Script/NavigationSystem.AbstractNavData" InputPin)
  (CallFunction|RemoveActorfromArraybyClass "/Script/Engine.WorldSettings" InputPin)
  (CallFunction|RemoveActorfromArraybyClass "/Script/Engine.SkyLight" InputPin)
  (Utilities|Array|RemoveIndex InputPin (- (Utilities|Array|Length InputPin) 1)))