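; BP_DummyCube is a configurable placeholder cube that displays a name label on its faces.
; The construction script scales the mesh holder, compensates text scale against Y and Z stretch, and tints the material through SurfaceColor.
; It also sets text color, toggles label pairs per axis, and rotates them unless ChangeDirection is set.
; RefreshMeshScale only stores a new MeshScale; an unconnected copy of the construction logic remains in the event graph.
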(event Custom|RefreshMeshScale
  (params (InMeshScale :type Vector))
  (Variables|MeshSetting|SetMeshScale InMeshScale))

(fn ConstructionScript
  (bind _textrender (Variables|Default|GetTextRender))
  (bind _meshscale (Variables|MeshSetting|GetMeshScale))
  (bind _textscale (Variables|Text|GetTextScale))
  (Transformation|SetRelativeScale3D (Variables|Default|GetMeshHolder) (Variables|MeshSetting|GetMeshScale))
  (Rendering|Components|TextRender|SetText _textrender (Variables|Default|GetName))
  (Transformation|SetRelativeScale3D (Variables|Default|GetTextRender3) (Math|Vector|MakeVector _textscale (/ _textscale (.y _meshscale)) (/ _textscale (.z _meshscale))))
  (Rendering|Components|TextRender|SetTextRenderColor _textrender (Variables|Text|GetTextColor))
  (Rendering|SetVisibility (Variables|Default|GetTextRender3) (Variables|Text|GetToggleX) false)
  (Rendering|SetVisibility (Variables|Default|GetTextRender) (Variables|Text|GetToggleY) false)
  (Rendering|SetVisibility (Variables|Default|GetTextRender4) (Variables|Text|GetToggleZ) false)
  (if (Variables|텍스트|GetChangeDirection)
    _
    (else
      (Transformation|AddRelativeRotation (Variables|Default|GetTextRender2) "0.000000,0.000000,90.000000" false false)
      (Transformation|AddRelativeRotation (Variables|Default|GetTextRender) "0.000000,0.000000,90.000000" false false)
      (Transformation|AddRelativeRotation (Variables|Default|GetTextRender4) "0.000000,90.000000,0.000000" false false)))
  (Rendering|Material|SetVectorParameterValueonMaterials (Variables|Default|GetStaticMesh) "SurfaceColor" (Math|Conversions|ToVector(LinearColor) (Variables|MeshSetting|GetColor))))