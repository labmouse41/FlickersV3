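; BP_SoundPlayer plays an escalating sequence of string sounds as flower hits are registered in quick succession.
; PlayFlowerSound advances ContinualFlowerCount on BP_MainGameState, resetting it first if over five seconds have passed since the previous call.
; The PlayFlowerHitSound macro selects one of eight strings by count, playing at world origin.
; The eighth adds a delayed RandomHarmony sound, then the count resets to zero.
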(event Custom|PlayFlowerSound
  (bind _bp_main_game_state (Variables|Default|GetBP%20Main%20Game%20State))
  (Variables|Default|SetCurrentTime (Utilities|Time|GetGameTimeinSeconds))
  (if (> (- (Variables|Default|GetCurrentTime) (Variables|Default|GetPast%20Time)) 5.0)
    (Variables|/Game/GameModes/BP_MainGameState.BP_MainGameState_C|SetContinualFlowerCount (Variables|Default|GetBP%20Main%20Game%20State) 0))
  (Variables|Default|SetPast%20Time (Variables|Default|GetCurrentTime))
  (Default|ContinualFlowerCounter _bp_main_game_state)
  (|PlayFlowerHitSound
    (:execute2
      (if (== 8 (Variables|/Game/GameModes/BP_MainGameState.BP_MainGameState_C|GetContinualFlowerCount _bp_main_game_state))
        (Variables|/Game/GameModes/BP_MainGameState.BP_MainGameState_C|SetContinualFlowerCount (Variables|Default|GetBP%20Main%20Game%20State) 0)))))

(event EventBeginPlay
  (bind _asbp_main_game_state (Utilities|Casting|CastToBP_MainGameState (Game|GetGameState)))
  (Variables|Default|SetBP%20Main%20Game%20State _asbp_main_game_state))

(fn ConstructionScript)