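; BP_StageMove records stage progression when its MovetoNextStage event fires, then returns the game to MainMenuMap.
; It loads the BP_SaveStage save slot and uses the current level name to set the following stage's Clear flag for Stage1 through Stage3.
; After a short delay it calls OpenLevel, then saves the slot.
; Stage4 does nothing, and a failed save cast stops the event.
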(event Custom|Move%20to%20Next%20Stage
  (bind _returnvalue (SaveGame|LoadGamefromSlot "BP_SaveStage"))
  (bind _asbp_save_stage (Utilities|Casting|CastToBP_SaveStage _returnvalue))
  (bind _returnvalue_2 (Game|GetCurrentLevelName true))
  (if (Utilities|Enum|Equal(Enum) _returnvalue_2 "Stage1")
    (Variables|/Game/Blueprints/BP_SaveStage.BP_SaveStage_C|SetStage%202%20Clear _asbp_save_stage true)
    (Utilities|FlowControl|Delay 2.0 :!label _label)
    (Game|OpenLevel(byName) "MainMenuMap")
    (SaveGame|SaveGametoSlot _asbp_save_stage "BP_SaveStage")
    (elif (Utilities|Enum|Equal(Enum) _returnvalue_2 "Stage2")
      (Variables|/Game/Blueprints/BP_SaveStage.BP_SaveStage_C|SetStage%203%20Clear _asbp_save_stage true)
      (goto _label)
      (elif (Utilities|Enum|Equal(Enum) _returnvalue_2 "Stage3")
        (Variables|/Game/Blueprints/BP_SaveStage.BP_SaveStage_C|SetStage%204%20Clear _asbp_save_stage true)
        (goto _label)
        (elif (Utilities|Enum|Equal(Enum) _returnvalue_2 "Stage4")
          _)))))

(fn ConstructionScript)