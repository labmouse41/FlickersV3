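; BP_CountingFlower keeps a tally of flowers per set tag and can trigger camera moves from it.
; Parallel arrays hold tags and totals, with EnlistFlowerSets adding to the count under the fixed "None" tag.
; FlowerMinusOne decrements only when the given tag lookup returns -1.
; If the recomputed count minus one equals -1, it calls MoveCamera on CamPos entries whose FlowerTag is "None".
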(event Custom|Enlist%20Flower%20Sets
  (bind _flowersettags (Variables|Default|GetFlowerSetTags))
  (bind _returnvalue (Utilities|Array|FindItem _flowersettags ""))
  (if (== _returnvalue -1)
    (Utilities|Array|Add (Variables|Default|GetFlowerSetTags) "")
    (Utilities|Array|Add (Variables|Default|GetFlowerSetTotalNumbers) 1)
    (else
      (Utilities|Array|SetArrayElem (Variables|Default|GetFlowerSetTotalNumbers) _returnvalue (+ (Utilities|Array|Get(acopy) (Variables|Default|GetFlowerSetTotalNumbers) _returnvalue) 1)))))

(event Custom|Flower%20Minus%20One
  (params (ItemToFind :type Name%20%28by%20ref%29))
  (bind _flowersettags (Variables|Default|GetFlowerSetTags))
  (bind _flowersettotalnumbers (Variables|Default|GetFlowerSetTotalNumbers))
  (bind _returnvalue (Utilities|Array|FindItem _flowersettags ItemToFind))
  (bind _output (Utilities|Array|Get(acopy) _flowersettotalnumbers _returnvalue))
  (bind _returnvalue_2 (+ _output -1))
  (if (== _returnvalue -1)
    (Utilities|Array|SetArrayElem (Variables|Default|GetFlowerSetTotalNumbers) _returnvalue _returnvalue_2)
    (if (== _returnvalue_2 -1)
      (for _array_element (Variables|Default|GetCamPos)
        (if (== (GameplayTags|GetTagName (Variables|/Game/Blueprints/BP_CamPos.BP_CamPos_C|GetFlowerTag _array_element)) "")
          (Default|MoveCamera _array_element))))))

(fn ConstructionScript)