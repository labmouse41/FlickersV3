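; BP_Observer is a player-controlled observer pawn that flies freely using Enhanced Input for look and movement.
; Look input drives yaw and pitch, while move input combines forward, strafe and world-vertical axes.
; A forward trace against WorldStatic blends the forward axis toward world up as geometry nears, with a power curve shaping the falloff.
; Left click is empty, and a material parameter collection toggle is left unconnected.
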(event Input|EnhancedActionEvents|EnhancedInputActionIA_Move
  (params (ActionValue :type Vector :default "0, 0, 0") (ElapsedSeconds :type Float%20%28double-precision%29) (TriggeredSeconds :type Float%20%28double-precision%29) (InputAction :type Input%20Action%20Object%20Reference :default "/Game/ThirdPerson/Input/Actions/IA_Move.IA_Move"))
  (bind _returnvalue (Pawn|GetControlRotation :!class /Script/Engine.Pawn))
  (bind _returnvalue_2 (Transformation|GetActorLocation))
  (bind _returnvalue_3 (Math|Vector|MakeVector 0.0 0.0 1.0))
  (Variables|Default|SetMovementInput ActionValue)
  (Variables|Default|SetControlForward (Math|Vector|GetForwardVector _returnvalue))
  (Variables|Default|SetControlRight (Math|Vector|GetRightVector _returnvalue))
  (bind _outhit (Collision|LineTraceForObjects _returnvalue_2 (+ _returnvalue_2 (* (Variables|Default|GetControlForward) 2048.0)) (Utilities|Array|MakeArray "ObjectTypeQuery1") false 0 "None" true "(R=1.000000,G=0.000000,B=0.000000,A=1.000000)" "(R=0.000000,G=1.000000,B=0.000000,A=1.000000)" 0.2))
  (Pawn|Input|AddMovementInput (+ (* (Class|KismetMathLibrary|VectorSlerpNormals _returnvalue_3 (Variables|Default|GetControlForward) (Math|Float|Max(Float) (+ (* (Math|Conversions|ToFloat(Boolean) (.bBlockingHit (Collision|BreakHitResult _outhit))) -1.0) 1.0) (Math|Float|Power (Math|Float|Clamp(Float) (/ (.Distance (Collision|BreakHitResult _outhit)) 2048.0)) 0.2))) (.y (Variables|Default|GetMovementInput))) (* (Variables|Default|GetControlRight) (.x (Variables|Default|GetMovementInput))) (* _returnvalue_3 (.z (Variables|Default|GetMovementInput)))) 1.0 false))

(event Input|EnhancedActionEvents|EnhancedInputActionIA_LeftClick
  (params (ActionValue :type Boolean) (ElapsedSeconds :type Float%20%28double-precision%29) (TriggeredSeconds :type Float%20%28double-precision%29) (InputAction :type Input%20Action%20Object%20Reference :default "/Game/ThirdPerson/Input/Actions/IA_LeftClick.IA_LeftClick")))

(event Input|EnhancedActionEvents|EnhancedInputActionIA_Look
  (params (ActionValue :type Vector%202D%20Structure) (ElapsedSeconds :type Float%20%28double-precision%29) (TriggeredSeconds :type Float%20%28double-precision%29) (InputAction :type Input%20Action%20Object%20Reference :default "/Game/ThirdPerson/Input/Actions/IA_Look.IA_Look"))
  (Pawn|Input|AddControllerYawInput (.x ActionValue))
  (Pawn|Input|AddControllerPitchInput (.y ActionValue)))

(event EventTick
  (params (DeltaSeconds :type Float%20%28single-precision%29))
  (Variables|Default|SetDeltaSeconds DeltaSeconds))

(event EventBeginPlay
  (bind _as플레이어_컨트롤러 (Utilities|Casting|CastToPlayerController (Pawn|GetController)))
  (Utilities|IsValid (PlayerController|LocalPlayerSubsystems|GetEnhancedInputLocalPlayerSubsystem _as플레이어_컨트롤러)
    (:Is%20Valid
      (Input|AddMappingContext (PlayerController|LocalPlayerSubsystems|GetEnhancedInputLocalPlayerSubsystem _as플레이어_컨트롤러) "/Game/ThirdPerson/Input/IMC_Default.IMC_Default" 0 "(bIgnoreAllPressedKeysUntilRelease=True,bForceImmediately=False,bNotifyUserSettings=False)"))))

(fn ConstructionScript)