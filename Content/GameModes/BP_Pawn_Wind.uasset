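; BP_Pawn_Wind is a floating pawn that feeds its movement into the windy grass material parameters.
; Each Tick it writes its location to the PlayerPos vector in the MPC_WindyGrass parameter collection.
; It also writes PlayerSpeedRate, its velocity length divided by the FloatingPawnMovement max speed, so materials using the collection can read relative speed.
; The left-click input event is present but empty.
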(event Input|EnhancedActionEvents|EnhancedInputActionIA_LeftClick
  (params (ActionValue :type Boolean) (ElapsedSeconds :type Float%20%28double-precision%29) (TriggeredSeconds :type Float%20%28double-precision%29) (InputAction :type Input%20Action%20Object%20Reference :default "/Game/ThirdPerson/Input/Actions/IA_LeftClick.IA_LeftClick")))

(event EventBeginPlay
  (|CallParentFunction))

(event EventTick
  (params (DeltaSeconds :type Float%20%28single-precision%29))
  (Rendering|Material|SetVectorParameterValue "/Game/Materials/ParameterCollection/MPC_WindyGrass.MPC_WindyGrass" "PlayerPos" (Math|Conversions|ToLinearColor(Vector) (Transformation|GetActorLocation)) :!class /Script/Engine.KismetMaterialLibrary)
  (Rendering|Material|SetScalarParameterValue "/Game/Materials/ParameterCollection/MPC_WindyGrass.MPC_WindyGrass" "PlayerSpeedRate" (/ (Math|Vector|VectorLength (Transformation|GetVelocity)) (Class|MovementComponent|GetMaxSpeed (Variables|Default|GetFloatingPawnMovement))) :!class /Script/Engine.KismetMaterialLibrary))

(fn ConstructionScript
  (|CallParentFunction))